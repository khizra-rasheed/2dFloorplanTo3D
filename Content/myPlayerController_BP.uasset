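; Player controller that binds hotkeys to image-driven cube commands on MyCharacter_BP, camera switching and an AI image widget.
; BeginPlay caches the character; key 1 rebuilds cubes from an image, and setKernelSize forwards kernel size to it.
; P alternates between viewing a CameraActor and possessing BP_ThirdPersonCharacter.
; V and B call the widget, but its creation and the local AI startup are unwired, leaving WidgetREF unassigned here.
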(event `self.ReceiveBeginPlay`
  (bind _returnvalue (`GameplayStatics.GetActorOfClass` "/Game/MyCharacter_BP.MyCharacter_BP_C"))
  (set `self.characterREF` _returnvalue))

(event `Key|One`
  (params (Key :type "Key Structure"))
  (bind _characterref (`self.characterREF`))
  (:`Pressed`
    (`/Game/MyCharacter_BP.delCubes` _characterref)
    (`/Game/MyCharacter_BP.readImg1` _characterref)))

(event `Key|P`
  (params (Key :type "Key Structure"))
  (:`Pressed`
    (`/Engine/EditorBlueprintResources/StandardMacros.FlipFlop`
      (:`A`
        (bind _returnvalue (`GameplayStatics.GetActorOfClass` "/Script/Engine.CameraActor"))
        (`self.SetViewTargetWithBlend` _returnvalue))
      (:`B`
        (bind _returnvalue_2 (`GameplayStatics.GetActorOfClass` "/Game/ThirdPerson/Blueprints/BP_ThirdPersonCharacter.BP_ThirdPersonCharacter_C"))
        (`self.Possess` _returnvalue_2)))))

(event `Key|V`
  (params (Key :type "Key Structure"))
  (:`Pressed`
    (`/Game/WBP_AI_imageGenWithPrompt.show widget'` (`self.widgetREF`))))

(event `Key|B`
  (params (Key :type "Key Structure"))
  (:`Pressed`
    (`/Game/WBP_AI_imageGenWithPrompt.CHECK FUNCTIONALITY` (`self.widgetREF`))))

(event `setKernelSize`
  (params (`Kernel Size` :type Integer))
  (`/Game/MyCharacter_BP.setkernel` (`self.characterREF`) `Kernel Size`))

(fn `UserConstructionScript`)