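; Player character Blueprint that turns an image into blocks, likely floor-plan walls, on the Bp_GridManager grid.
; readImg1 passes the image, a YOLO ONNX model path and KernelSize to ReadImageBP, clears old cubes, then spawns one stretched Cube per BoxData run.
; Door and corner-marker spawning from DoorArr and DoorCorners is present but disconnected.
; The construction script builds a procedural mesh section from stored vertices and triangles.
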(event `self.ReceiveBeginPlay`
  (bind _returnvalue (`GameplayStatics.GetActorOfClass` "/Game/GridPlane/Bluepritns/Bp_GridManager.Bp_GridManager_C"))
  (set `self.gridRef` _returnvalue)
  (bind _asmy_player_controller_bp (cast `/Game/myPlayerController_BP` (`self.GetController`)))
  (set `self.As My Player Controller BP` _asmy_player_controller_bp))

(event `self.ReceiveTick`
  (params (DeltaSeconds :type "Float (single-precision)")))

(event `delCubes`
  (bind _outactors (`GameplayStatics.GetAllActorsOfClass` "/Game/cube.cube_C"))
  (for _array_element _outactors
    (`self.K2_DestroyActor` _array_element)
    (`KismetArrayLibrary.Array_Clear` (`self.rows`))
    (`KismetArrayLibrary.Array_Clear` (`self.cols`))
    (`BlueprintMapLibrary.Map_Clear` (`self.WallMap`)))
  (bind _outactors_2 (`GameplayStatics.GetAllActorsOfClass` "/Game/windowsCube.windowsCube_C"))
  (for _array_element_2 _outactors_2
    (`self.K2_DestroyActor` _array_element_2)))

(event `readImg1`
  (`KismetSystemLibrary.PrintString` "Hello")
  (`self.ReadImageBP` "images/img.png" "images/yolo_objDet.onnx" (`self.Kernel Size`))
  (`self.delCubes`)
  (for _array_element (`self.boxData`)
    (bind _output (`|GetArrayItem` (`.Rows` (break `BlackPixelRange` _array_element))))
    (bind (_istilevalid_ _gridlocation) (`/Game/GridPlane/Bluepritns/Bp_GridManager.TileToGridLocation` (`self.gridRef`) (+ (break `BlackPixelRange` _array_element) (`self.colsToEscape`)) (+ _output (`self.rowsToEscape`)) false))
    (bind _output_get (set `self.Spawn Transform Scale X` (`KismetMathLibrary.Conv_IntToDouble` (* (- (`.End` (break `BlackPixelRange` _array_element)) (break `BlackPixelRange` _array_element)) 2))))
    (if (== _output_get 0.0)
      (set `self.Spawn Transform Scale X` 2.0))
    (bind _output_get_2 (set `self.Spawn Transform Scale Y` (`KismetMathLibrary.Conv_IntToDouble` (* (+ (- (`|GetArrayItem` (`.Rows` (break `BlackPixelRange` _array_element)) (- (`KismetArrayLibrary.Array_Length` (`.Rows` (break `BlackPixelRange` _array_element))) 1)) _output) 1) 2))))
    (if (== _output_get_2 0.0)
      (set `self.Spawn Transform Scale Y` 2.0))
    (`|SpawnActorFromClass` "/Game/cube.cube_C" (`KismetMathLibrary.MakeTransform` (`KismetMathLibrary.MakeVector` (`KismetMathLibrary.BreakVector2D` _gridlocation) (`.Y` (`KismetMathLibrary.BreakVector2D` _gridlocation))) (struct) (`KismetMathLibrary.MakeVector` (`self.Spawn Transform Scale X`) (`self.Spawn Transform Scale Y`) 50.0)) "Undefined" "OverrideRootScale" null null)))

(event `setkernel`
  (params (`Kernel Size` :type Integer))
  (set `self.Kernel Size` `Kernel Size`))

(fn `UserConstructionScript`
  (`ProceduralMeshComponent.CreateMeshSection_LinearColor` :`self` (`self.ProceduralMesh`) :`Vertices` (`self.Vertices`) :`Triangles` (`self.Triangles`)))